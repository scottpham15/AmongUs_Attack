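; Gameplay Ability that lets a wizard attack a nearby crewmate in a multiplayer imposter-style game.
; On activation it commits, starts the attack montage and immediately runs a debug-drawn sphere overlap around the avatar for other wizard pawns.
; The first wizard found receives GE_ReduceHealth, but the ability cancels if that wizard is an imposter or none is found.
; The ability ends when the montage completes, blends out or is interrupted.
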(event Ability|EventActivateAbility
  (bind _returnvalue (Ability|GetAvatarActorfromActorInfo))
  (bind _returnvalue_2 (Transformation|GetActorLocation _returnvalue))
  (Ability|CommitAbility)
  (|PlayMontageandWaitProxy "None" "/Game/BattleWizardPolyart/AM_AttackWizard.AM_AttackWizard" 1.0 "None" true 1.0 0.0 false
    (:then
      (Rendering|Debug|DrawDebugSphere _returnvalue_2 2e+02 12 "(R=1.000000,G=0.000000,B=0.376997,A=1.000000)" 0.0)
      (bind (_outactors _returnvalue_3) (Collision|SphereOverlapActors _returnvalue_2 2e+02 (Utilities|Array|MakeArray "ObjectTypeQuery3") "/Game/Multiplayer/Blueprint_Wizard/BP_WizardCharacter.BP_WizardCharacter_C" (Utilities|Array|MakeArray _returnvalue)))
      (if _returnvalue_3
        (bind _asbp_wizard_character (Utilities|Casting|CastToBP_WizardCharacter (Utilities|Array|Get(acopy) _outactors)))
        (if (Variables|/Game/Multiplayer/Blueprint_Wizard/BP_WizardCharacter.BP_WizardCharacter_C|GetbImposter _asbp_wizard_character)
          (Ability|CancelAbility :!label _label)
          (else
            (GameplayEffects|ApplyGameplayEffectSpecToSelf (Ability|GetAbilitySystemComponent (Utilities|Array|Get(acopy) _outactors)) (Ability|MakeOutgoingGameplayEffectSpec "/Game/Multiplayer/Blueprint_Wizard/GE_ReduceHealth.GE_ReduceHealth_C"))))
        (else
          (goto _label))))
    (:OnCompleted
      (Ability|EndAbility :!label _label_2))
    (:OnBlendOut
      (goto _label_2))
    (:OnInterrupted
      (goto _label_2))
    (:OnCancelled
      (goto _label_2))))