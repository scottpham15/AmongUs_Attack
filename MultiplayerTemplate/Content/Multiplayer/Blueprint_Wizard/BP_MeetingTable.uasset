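; BP_MeetingTable is a multiplayer meeting table actor that offers a use button to wizard players who come near it.
; A Sphere overlap casts the entering actor to BP_WizardCharacter, then its controller to BP_WizardController, and calls TurnOnUseButton if ReportBTN is valid.
; Leaving the sphere calls TurnOffUseButton on that controller without the validity check.
; The table itself holds no meeting logic.
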(event OnComponentBeginOverlap(Sphere)
  (params (OverlappedComponent :type Primitive%20Component%20Object%20Reference) (OtherActor :type Actor%20Object%20Reference) (OtherComp :type Primitive%20Component%20Object%20Reference) (OtherBodyIndex :type Integer) (bFromSweep :type Boolean) (SweepResult :type Hit%20Result%20Structure%20%28by%20ref%29))
  (bind _asbp_wizard_character (Utilities|Casting|CastToBP_WizardCharacter OtherActor))
  (bind _asbp_wizard_controller (Utilities|Casting|CastToBP_WizardController (Pawn|GetController _asbp_wizard_character)))
  (Utilities|IsValid (Variables|/Game/Multiplayer/Blueprint_Wizard/BP_WizardController.BP_WizardController_C|GetReportBTN _asbp_wizard_controller)
    (:Is%20Valid
      (Default|TurnonUseButton _asbp_wizard_controller))))

(event OnComponentEndOverlap(Sphere)
  (params (OverlappedComponent :type Primitive%20Component%20Object%20Reference) (OtherActor :type Actor%20Object%20Reference) (OtherComp :type Primitive%20Component%20Object%20Reference) (OtherBodyIndex :type Integer))
  (bind _asbp_wizard_character (Utilities|Casting|CastToBP_WizardCharacter OtherActor))
  (bind _asbp_wizard_controller (Utilities|Casting|CastToBP_WizardController (Pawn|GetController _asbp_wizard_character)))
  (Default|TurnOffUseButton _asbp_wizard_controller))

(event EventBeginPlay)

(event Collision|EventActorBeginOverlap
  (params (OtherActor :type Actor%20Object%20Reference)))

(event EventTick
  (params (DeltaSeconds :type Float%20%28single-precision%29)))

(fn ConstructionScript)